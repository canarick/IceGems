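; GemBP is a collectible gem actor that the player's ShipBP picks up by collision or by a collect event.
; Each Tick it toggles a custom-depth glow when the player pawn is within range and binds its Collect handler to the first ShipBP's dispatcher.
; Collect destroys the gem only if the player is in range.
; A ship hit on GemCollider destroys it and calls GemCollected, which the Collect path does not call.
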(event `self.ReceiveTick`
  (params (DeltaSeconds :type "Float (single-precision)"))
  ;[1 1 1] Glow
  (`PrimitiveComponent.SetRenderCustomDepth` (`self.Gem`) (<= (`KismetMathLibrary.Vector_Distance` (`self.K2_GetActorLocation`) (`self.K2_GetActorLocation` (`GameplayStatics.GetPlayerPawn` 0))) 60.0))
  ;[1 1 1] Collect
  ;;[1 1 1] Collect with Keypress
  (bind _outactors (`GameplayStatics.GetAllActorsOfClass` "/Game/Blueprints/ShipBP.ShipBP_C"))
  (add `/Game/Blueprints/ShipBP.Collect` (`|GetArrayItem` _outactors) (delegate `Collect`)))

(event `self.ReceiveBeginPlay`
  ;[1 1 1] Allow Gem to get Player Input
  (`self.EnableInput` (`GameplayStatics.GetPlayerController` 0)))

(event `Collect`
  ;[1 1 1] Collect
  ;;[1 1 1] Collect with Keypress
  (if (<= (`KismetMathLibrary.Vector_Distance` (`self.K2_GetActorLocation`) (`self.K2_GetActorLocation` (`GameplayStatics.GetPlayerPawn` 0))) 60.0)
    (`self.K2_DestroyActor`)))

(event `self.GemCollider.OnComponentHit`
  (params (HitComponent :type "PrimitiveComponent Object Reference") (OtherActor :type "Actor Object Reference") (OtherComp :type "PrimitiveComponent Object Reference") (NormalImpulse :type "Vector Structure") (Hit :type "HitResult Structure (by ref)"))
  ;[1 1 1] Collect
  ;;[1 1 1] Collect with Collision
  (cast `/Game/Blueprints/ShipBP` OtherActor)
  (`self.K2_DestroyActor`)
  (`self.GemCollected`))

(fn `UserConstructionScript`)