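; Global actor that manages a Score, raised by collected gems and spent by ship movement.
; Every Tick it binds to each GemBP's collected event and, inside that same loop, to the first ShipBP's move-forward and turn events.
; Gem pickups add points while Score is under a cap; moving and turning share a looped decrement that stops at zero, with turns costing less.
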(event `DecrementForward`
  (bind _score (`self.Score`))
  ;[1 1 1] Decrement Score
  ;;[1 1 1] Move Forward
  (for _ (range 5)
    (if (> _score 0) :!label _label
      (set `self.Score` (- _score 1)))))

(event `self.ReceiveTick`
  (params (DeltaSeconds :type "Float (single-precision)"))
  ;[1 1 1] Get Gems
  (bind _outactors (`GameplayStatics.GetAllActorsOfClass` "/Game/Blueprints/GemBP.GemBP_C"))
  (for _array_element _outactors
    (add `/Game/Blueprints/GemBP.GemCollected` _array_element (delegate `IncrementScore`))
    (bind _outactors_2 (`GameplayStatics.GetAllActorsOfClass` "/Game/Blueprints/ShipBP.ShipBP_C"))
    (bind _output (`|GetArrayItem` _outactors_2))
    ;[1 1 1] Decrement Score
    ;;[1 1 1] Move Forward
    (add `/Game/Blueprints/ShipBP.MoveForward` _output (delegate `DecrementForward`))
    ;;[1 1 1] Turn
    (add `/Game/Blueprints/ShipBP.Turn` _output (delegate `DecrementTurn`))))

(event `self.ReceiveBeginPlay`
  ;[1 1 1] Allow Global to get Player Input
  (`self.EnableInput` (`GameplayStatics.GetPlayerController` 0)))

(event `IncrementScore`
  (bind _score (`self.Score`))
  ;[1 1 1] Increment Score
  (if (< _score 100)
    (set `self.Score` (+ _score 10))))

(event `DecrementTurn`
  ;[1 1 1] Decrement Score
  ;;[1 1 1] Turn
  (for _ (range 2)
    (goto _label)))

(fn `UserConstructionScript`)