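; Boss enemy pawn that wanders the level and wins the game for the player when shot down.
; A self-recalling event moves it to random nearby navmesh points, pausing after each successful move.
; Projectile overlaps play an explosion sound and increment a hit counter stored on a Global actor.
; Once the counter exceeds its threshold, the next hit starts an animation, sets GameWon on Global and immediately destroys the boss.
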(event `self.ReceiveBeginPlay`
  (`self.MoveToRamdomLocation`))

(event `self.ReceiveActorBeginOverlap`
  (params (OtherActor :type "Actor Object Reference"))
  (cast `/Game/Blueprints/FirstPersonProjectile` OtherActor)
  (bind _outactors (`GameplayStatics.GetAllActorsOfClass` "/Game/Blueprints/Global.Global_C"))
  (if (> (`/Game/Blueprints/Global.bossHit` (`|GetArrayItem` _outactors)) 2.0)
    (`SkeletalMeshComponent.PlayAnimation` (`self.Mesh`) null false)
    (bind _outactors_2 (`GameplayStatics.GetAllActorsOfClass` "/Game/Blueprints/Global.Global_C"))
    (set `/Game/Blueprints/Global.gameWon` true (`|GetArrayItem` _outactors_2))
    (`self.K2_DestroyActor`)
    (else
      (bind _outactors_3 (`GameplayStatics.GetAllActorsOfClass` "/Game/Blueprints/Global.Global_C"))
      (bind _output (`|GetArrayItem` _outactors_3))
      (set `/Game/Blueprints/Global.bossHit` (+ (`/Game/Blueprints/Global.bossHit` _output) 1.0) _output)
      (`GameplayStatics.PlaySoundAtLocation` "/Game/StarterContent/Audio/Explosion01.Explosion01" (`SceneComponent.K2_GetComponentLocation` (`self.Mesh`)) (struct) 1.0 1.0 0.0 null null null))))

(event `MoveToRamdomLocation`
  (`|AIMoveTo` self (`NavigationSystemV1.K2_GetRandomLocationInNavigableRadius` (`self.K2_GetActorLocation`) 500.0 null null) null
    (:`then`
      (`KismetSystemLibrary.Delay` 2.0)
      (`self.MoveToRamdomLocation`))))

(fn `UserConstructionScript`)