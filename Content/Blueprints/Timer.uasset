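; Timer Blueprint that runs a repeating countdown and triggers a roar each time it expires.
; BeginPlay starts a looping one-second timer that runs Decrement to lower the Time variable.
; With five seconds left, it spawns the Roar sound at the world origin as an advance cue.
; On reaching zero, it invokes CallRoar and resets the countdown to thirty seconds.
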(event `self.ReceiveBeginPlay`
  (`KismetSystemLibrary.K2_SetTimer` null "Decrement" 1.0 true))

(fn `Decrement`
  (bind _returnvalue (- (`self.Time`) 1))
  (if (<= _returnvalue 0)
    (`self.Roar`)
    (set `self.Time` 30)
    (else
      (bind _output_get (set `self.Time` _returnvalue))
      (if (== _output_get 5)
        (`GameplayStatics.SpawnSoundAtLocation` "/Game/StarterContent/Audio/roar.roar" (0.0 0.0 0.0) (struct) 1.0 1.0 0.0 null null)))))

(fn `UserConstructionScript`)