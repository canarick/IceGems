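; AI character that wanders the navmesh at random and is destroyed when hit by a first-person projectile.
; From BeginPlay, a self-calling event issues AI Move To toward a random navigable point around its current location.
; The loop runs off the immediate exec pin, so it retargets after a short delay without waiting for arrival.
; Overlapping a projectile plays an explosion sound at the mesh and destroys the actor.
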(event `self.ReceiveBeginPlay`
  (`self.MoveToRamdomLocation`))

(event `self.ReceiveActorBeginOverlap`
  (params (OtherActor :type "Actor Object Reference"))
  (cast `/Game/Blueprints/FirstPersonProjectile` OtherActor)
  (`GameplayStatics.PlaySoundAtLocation` "/Game/StarterContent/Audio/Explosion01.Explosion01" (`SceneComponent.K2_GetComponentLocation` (`self.Mesh`)) (struct) 1.0 1.0 0.0 null null null)
  (`self.K2_DestroyActor`))

(event `MoveToRamdomLocation`
  (`|AIMoveTo` self (`NavigationSystemV1.K2_GetRandomLocationInNavigableRadius` (`self.K2_GetActorLocation`) 500.0 null null) null
    (:`then`
      (`KismetSystemLibrary.Delay` 2.0)
      (`self.MoveToRamdomLocation`))))

(fn `UserConstructionScript`)